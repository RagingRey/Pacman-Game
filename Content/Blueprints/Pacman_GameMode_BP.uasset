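; Game mode for a Pac-Man game that sets up the level and handles the win condition.
; BeginPlay blends the view to the first CameraActor found, adds the HUD widget, then unfreezes the Pac-Man pawn after a short delay.
; Tick counts remaining Food actors by searching the level every frame.
; At zero food it adds the win widget, repeatedly since nothing guards it, and opens Level_01 after a delay.
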(event Custom|InitializeCamera
  ;[1 1 1] Find And Initiate Camera
  (bind _outactors (Actor|GetAllActorsOfClass "/Script/Engine.CameraActor"))
  (Game|Player|SetViewTargetwithBlend (Game|GetPlayerController 0) (Utilities|Array|Get(acopy) _outactors) 1.0 "VTBlend_Linear" 0.0 false))

(event Custom|Get%20Food
  ;[1 1 1] Get Food Count
  (bind _outactors (Actor|GetAllActorsOfClass "/Script/Pacman.Food"))
  (Variables|Default|SetFoods%20Remaining (Utilities|Array|Length _outactors)))

(event Custom|Add%20Widget
  ;[1 1 1] Add Pacman UI Widget
  (bind _returnvalue (UserInterface|CreateWidget "/Game/Blueprints/UI/Pacman_Widget_BP.Pacman_Widget_BP_C"))
  (UserInterface|Viewport|AddtoViewport _returnvalue 0))

(event Custom|You%20WIn
  ;[1 1 1] If Player Wins
  (bind _output_get (Variables|Default|SetFoods%20Remaining (Variables|Default|GetFoods%20Remaining)))
  (bind _output_get_2 (Variables|Default|SetNo%20Food (== _output_get 0)))
  (if _output_get_2
    (bind _returnvalue (UserInterface|CreateWidget "/Game/Blueprints/UI/YouWin_Widget_BP.YouWin_Widget_BP_C"))
    (UserInterface|Viewport|AddtoViewport _returnvalue 0)
    (Utilities|FlowControl|Delay 3.0)
    (Game|OpenLevel(byName) "Level_01")))

(event EventBeginPlay
  (CallFunction|InitializeCamera)
  (CallFunction|AddWidget)
  (Utilities|FlowControl|Delay 2.0)
  (bind _aspacman_pawn_bp (Utilities|Casting|CastToPacmanPawn_BP (Game|Player|GetPlayerPawn 0)))
  (Class|PacmanPawn|SetFrozen _aspacman_pawn_bp false))

(event EventTick
  (params (DeltaSeconds :type Float%20%28single-precision%29))
  (CallFunction|GetFood)
  (CallFunction|YouWin))

(fn ConstructionScript)